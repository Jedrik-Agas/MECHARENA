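; AC_HealthSystem is a health component that tracks damage taken by its owning actor and reports hits and death.
; On BeginPlay it fills CurrentHealth from MaxHealth and binds to the owner's OnTakeAnyDamage.
; Each damage event subtracts from health and broadcasts OnHit with the new value and percent, followed by OnDeath at zero or below.
; Health is not clamped, and OnDeath can fire again on later hits.
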(event `self.ReceiveBeginPlay`
  (set `self.CurrentHealth` (`self.MaxHealth`))
  (add `Actor.OnTakeAnyDamage` (`self.GetOwner`) (delegate `Take Damage`)))

(event `Take Damage`
  (params (DamagedActor :type "Actor Object Reference") (Damage :type "Float (single-precision)") (DamageType :type "DamageType Object Reference") (InstigatedBy :type "Controller Object Reference") (DamageCauser :type "Actor Object Reference"))
  (bind _output_get (set `self.CurrentHealth` (- (`self.CurrentHealth`) Damage)))
  (if (<= _output_get 0.0)
    (`self.OnHit` (`self.CurrentHealth`) (/ (`self.CurrentHealth`) (`self.MaxHealth`)))
    (`self.OnDeath`)
    (else
      (`self.OnHit` (`self.CurrentHealth`) (/ (`self.CurrentHealth`) (`self.MaxHealth`))))))