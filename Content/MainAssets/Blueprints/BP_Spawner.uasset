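; BP_Spawner is a wave spawner that places BP_MechEnemy actors at random points inside its Box bounds.
; It spawns a wave one second after BeginPlay and whenever BP_ThirdPersonGameMode fires NextWave, growing each wave by one enemy.
; When the wave counter equals DivisibleBy5 and the player lacks tactical armor, it also spawns BP_Tactical_Armor in the box.
; That threshold advances by five only when armor spawns.
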(event `self.ReceiveBeginPlay`
  (`KismetSystemLibrary.Delay` 1.0)
  (bind _asbp_third_person_game_mode (cast `/Game/MainAssets/CharacterBlueprints/BP_ThirdPersonGameMode` (`GameplayStatics.GetGameMode`)))
  (add `/Game/MainAssets/CharacterBlueprints/BP_ThirdPersonGameMode.NextWave` _asbp_third_person_game_mode (delegate `SpawnEnemy`))
  (`self.SpawnEnemy`))

(event `SpawnEnemy`
  (bind (_origin _boxextent) (`KismetSystemLibrary.GetComponentBounds` (`self.Box`)))
  (bind (_origin_2 _boxextent_2) (`KismetSystemLibrary.GetComponentBounds` (`self.Box`)))
  (`|ExecutionSequence`
    (:`then_0`
      (for _ (range (+ (`self.EnemiesSpawned`) 1))
        (`|SpawnActorFromClass` "/Game/MainAssets/Blueprints/BP_MechEnemy.BP_MechEnemy_C" (`KismetMathLibrary.Conv_VectorToTransform` (`KismetMathLibrary.RandomPointInBoundingBox` _origin _boxextent)) "AdjustIfPossibleButAlwaysSpawn" "MultiplyWithRoot" null null))
      (bind _result (`/Engine/EditorBlueprintResources/StandardMacros.IncrementInt` (`self.EnemiesSpawned`))
        (:`  `
          (set `self.EnemiesSpawned` _result))))
    (:`then_1`
      (if (== (`self.EnemiesSpawned`) (`self.Divisible by 5?`))
        (bind _returnvalue (`GameplayStatics.GetActorOfClass` "/Game/MainAssets/CharacterBlueprints/BP_PlayerCharacter.BP_PlayerCharacter_C"))
        (if (not (`/Game/MainAssets/CharacterBlueprints/BP_PlayerCharacter.TAequipped` _returnvalue))
          (`|SpawnActorFromClass` "/Game/MainAssets/Blueprints/BP_Tactical_Armor.BP_Tactical_Armor_C" (`KismetMathLibrary.Conv_VectorToTransform` (`KismetMathLibrary.RandomPointInBoundingBox` _origin_2 _boxextent_2)) "AdjustIfPossibleButAlwaysSpawn" "MultiplyWithRoot" null null)
          (set `self.Divisible by 5?` (+ (`self.Divisible by 5?`) 5)))))))

(fn `UserConstructionScript`)