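; BP_HITTEST is a respawning target mech that displays its current health and reacts to death from its health system component.
; Hits update a text render with the new health value.
; On death it plays explosion effects and sound, hides the mesh and text, then once spawns an ammo pickup and opens the first BP_DOOR found.
; After a short delay it spawns a fresh copy of itself at the same transform, then destroys itself.
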(event `self.ReceiveBeginPlay`
  (add `/Game/MainAssets/CharacterBlueprints/AC_HealthSystem.OnHit` (`self.AC_HealthSystem`) (delegate `Hit`)))

(event `Hit`
  (params (`New Health Value` :type "Float (double-precision)") (`New Health Percent` :type "Float (double-precision)"))
  (bind _output_get (set `/Game/MainAssets/CharacterBlueprints/AC_HealthSystem.CurrentHealth` `New Health Value` (`self.AC_HealthSystem`)))
  (`TextRenderComponent.K2_SetText` (`self.TextRender`) (`KismetTextLibrary.Conv_StringToText` (`KismetStringLibrary.Conv_Int64ToString` (`KismetMathLibrary.Conv_DoubleToInt64` _output_get)))))

(event `self.AC_HealthSystem.OnDeath`
  (`ActorComponent.Activate` (`self.NS_Explosion`) false)
  (`SceneComponent.SetHiddenInGame` (`self.SM_Basic-Mech`) true false)
  (`SceneComponent.SetHiddenInGame` (`self.TextRender`) true false)
  (`GameplayStatics.SpawnSound2D` "/Game/StarterContent/Audio/Explosion01.Explosion01" 1.0 1.0 0.0 null)
  (`/Engine/EditorBlueprintResources/StandardMacros.DoOnce` false
    (:`Completed`
      (`|SpawnActorFromClass` "/Game/MainAssets/Blueprints/BP_Ammo.BP_Ammo_C" (`self.GetTransform`) "AdjustIfPossibleButAlwaysSpawn" "MultiplyWithRoot" null null)
      (`|ExecutionSequence`
        (:`then_0`
          (bind _returnvalue (`GameplayStatics.GetActorOfClass` "/Game/MainAssets/Blueprints/BP_DOOR.BP_DOOR_C"))
          (`/Game/MainAssets/Blueprints/BP_DOOR.OpenDoor` _returnvalue))
        (:`then_1`
          (`KismetSystemLibrary.Delay` 2.0)
          (`|SpawnActorFromClass` "BP_HITTEST_C" (`self.GetTransform`) "AdjustIfPossibleButAlwaysSpawn" "MultiplyWithRoot" null null))
        (:`then_2`
          (`KismetSystemLibrary.Delay` 2.1)
          (`self.K2_DestroyActor`))))))

(fn `UserConstructionScript`)