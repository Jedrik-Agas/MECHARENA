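; BP_Bullet is a projectile actor that damages the player character on contact.
; Its collision sphere's begin-overlap event ignores other actors and spawns an explosion emitter at the bullet when it hits the player.
; It then reads the shield flag on BP_PlayerCharacter, applying damage only if the shield is down, and destroys itself either way.
; A physics-simulation check on the overlapped component has empty branches and no effect.
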(event `self.SphereCollision.OnComponentBeginOverlap`
  (params (OverlappedComponent :type "PrimitiveComponent Object Reference") (OtherActor :type "Actor Object Reference") (OtherComp :type "PrimitiveComponent Object Reference") (OtherBodyIndex :type Integer) (bFromSweep :type Boolean) (SweepResult :type "HitResult Structure (by ref)"))
  (if (== OtherActor (`GameplayStatics.GetPlayerCharacter` 0))
    (if (`SceneComponent.IsSimulatingPhysics` OtherComp "None")
      _
      (else
        _))
    (`GameplayStatics.SpawnEmitterAtLocation` "/Game/StarterContent/Particles/P_Explosion.P_Explosion" (`self.K2_GetActorLocation`) (struct) (1.0 1.0 1.0) false)
    (bind _asbp_player_character (cast `/Game/MainAssets/CharacterBlueprints/BP_PlayerCharacter` (`GameplayStatics.GetPlayerCharacter` 0)))
    (if (`/Game/MainAssets/CharacterBlueprints/BP_PlayerCharacter.ShieldUp` _asbp_player_character)
      (`self.K2_DestroyActor`)
      (else
        (`GameplayStatics.ApplyDamage` _asbp_player_character 1.0 null self)
        (`self.K2_DestroyActor`)))))

(fn `UserConstructionScript`)