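; Mech enemy that chases the player via a self-restarting AI MoveTo and reports itself to the game mode's living-enemy count.
; Pawn sensing snaps it toward a seen player and fires a bullet from an arrow component with sound.
; Health component death hides the mesh, plays explosion effects and drops ammo once.
; After a delay it destroys itself, updates the enemy count and awards score based on player shield, defensive and shooting state.
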(event `self.ReceiveBeginPlay`
  (`|ExecutionSequence`
    (:`then_0`
      (bind _asbp_third_person_game_mode (cast `/Game/MainAssets/CharacterBlueprints/BP_ThirdPersonGameMode` (`GameplayStatics.GetGameMode`)))
      (`/Engine/EditorBlueprintResources/StandardMacros.IncrementInt` (`/Game/MainAssets/CharacterBlueprints/BP_ThirdPersonGameMode.EnemiesAlive` _asbp_third_person_game_mode)))
    (:`then_1`
      (add `/Game/MainAssets/CharacterBlueprints/AC_HealthSystem.OnHit` (`self.AC_HealthSystem`) (delegate `Hit`))
      (`self.Movement`))))

(event `Hit`
  (params (`New Health Value` :type "Float (double-precision)") (`New Health Percent` :type "Float (double-precision)"))
  (set `/Game/MainAssets/CharacterBlueprints/AC_HealthSystem.CurrentHealth` `New Health Value` (`self.AC_HealthSystem`)))

(event `self.PawnSensing.OnSeePawn`
  (params (Pawn :type "Pawn Object Reference"))
  (bind _returnvalue (`self.K2_GetActorLocation`))
  (bind _asbp_player_character (cast `/Game/MainAssets/CharacterBlueprints/BP_PlayerCharacter` Pawn))
  (`self.K2_SetActorRotation` (`KismetMathLibrary.FindRelativeLookAtRotation` (`KismetMathLibrary.Conv_VectorToTransform` _returnvalue) (`self.K2_GetActorLocation` _asbp_player_character)))
  (`|SpawnActorFromClass` "/Game/MainAssets/Blueprints/BP_Bullet.BP_Bullet_C" (`SceneComponent.K2_GetComponentToWorld` (`self.Bullet Arrow`)) "AdjustIfPossibleButAlwaysSpawn" "MultiplyWithRoot" null null)
  (`GameplayStatics.SpawnSoundAtLocation` "/Game/MainAssets/Audio/shotgun-fire.shotgun-fire" _returnvalue (struct) 1.0 1.0 0.0 null null))

(event `self.AC_HealthSystem.OnDeath`
  (`ActorComponent.Activate` (`self.NS_Explosion`) false)
  (`SceneComponent.SetHiddenInGame` (`self.SM_Basic-Mech`) true true)
  (`GameplayStatics.SpawnSoundAtLocation` "/Game/StarterContent/Audio/Explosion02.Explosion02" (`self.K2_GetActorLocation`) (struct) 1.0 1.0 0.0 null null)
  (`|ExecutionSequence`
    (:`then_0`
      (`KismetSystemLibrary.Delay` 1.0)
      (`self.K2_DestroyActor`)
      (bind _asbp_third_person_game_mode (cast `/Game/MainAssets/CharacterBlueprints/BP_ThirdPersonGameMode` (`GameplayStatics.GetGameMode`)))
      (`/Engine/EditorBlueprintResources/StandardMacros.DecrementInt` (`/Game/MainAssets/CharacterBlueprints/BP_ThirdPersonGameMode.EnemiesAlive` _asbp_third_person_game_mode)
        (:`  `
          (`/Game/MainAssets/CharacterBlueprints/BP_ThirdPersonGameMode.EnemiesLeft` _asbp_third_person_game_mode)
          (bind _asbp_player_character (cast `/Game/MainAssets/CharacterBlueprints/BP_PlayerCharacter` (`GameplayStatics.GetPlayerCharacter` 0)))
          (if (`/Game/MainAssets/CharacterBlueprints/BP_PlayerCharacter.ShieldUp` _asbp_player_character)
            (if (`/Game/MainAssets/CharacterBlueprints/BP_PlayerCharacter.Defenssive` _asbp_player_character)
              (set `/Game/MainAssets/CharacterBlueprints/BP_PlayerCharacter.SCORE` (+ (`/Game/MainAssets/CharacterBlueprints/BP_PlayerCharacter.SCORE` _asbp_player_character) 300) _asbp_player_character)
              (else
                (set `/Game/MainAssets/CharacterBlueprints/BP_PlayerCharacter.SCORE` (+ (`/Game/MainAssets/CharacterBlueprints/BP_PlayerCharacter.SCORE` _asbp_player_character) 500) _asbp_player_character)))
            (elif (`/Game/MainAssets/CharacterBlueprints/BP_PlayerCharacter.CanShoot` _asbp_player_character)
              (set `/Game/MainAssets/CharacterBlueprints/BP_PlayerCharacter.SCORE` (+ (`/Game/MainAssets/CharacterBlueprints/BP_PlayerCharacter.SCORE` _asbp_player_character) 100) _asbp_player_character)
              (else
                (set `/Game/MainAssets/CharacterBlueprints/BP_PlayerCharacter.SCORE` (+ (`/Game/MainAssets/CharacterBlueprints/BP_PlayerCharacter.SCORE` _asbp_player_character) 200) _asbp_player_character)))))))
    (:`then_1`
      (`/Engine/EditorBlueprintResources/StandardMacros.DoOnce` false
        (:`Completed`
          (`|SpawnActorFromClass` "/Game/MainAssets/Blueprints/BP_Ammo.BP_Ammo_C" (`self.GetTransform`) "AdjustIfPossibleButAlwaysSpawn" "MultiplyWithRoot" null null))))))

(event `Movement`
  (`|AIMoveTo` self (0.0 0.0 0.0) (`GameplayStatics.GetPlayerCharacter` 0)
    (:`OnSuccess`
      _)
    (:`OnFail`
      _))
  (`self.Movement`))

(fn `UserConstructionScript`)