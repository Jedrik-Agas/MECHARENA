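; Arena boundary actor that punishes the player for staying outside its box by applying damage when a countdown expires.
; Ending overlap starts a looping timer that drains the countdown; beginning overlap resets it to three seconds and makes the timer one-shot.
; At zero, a DoOnce deals 100 damage to the player character.
; It creates an arena UI widget, passes itself to it and calls ViewTime on each overlap change.
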(event `self.ReceiveBeginPlay`
  (bind _returnvalue (`|CreateWidget` "/Game/MainAssets/CharacterBlueprints/WBP_Arena_UI.WBP_Arena_UI_C" (`GameplayStatics.GetPlayerController` 0)))
  (set `self.ArenaUIRef` _returnvalue)
  (set `/Game/MainAssets/CharacterBlueprints/WBP_Arena_UI.BoundaryRef` self _returnvalue))

(event `self.Box.OnComponentBeginOverlap`
  (params (OverlappedComponent :type "PrimitiveComponent Object Reference") (OtherActor :type "Actor Object Reference") (OtherComp :type "PrimitiveComponent Object Reference") (OtherBodyIndex :type Integer) (bFromSweep :type Boolean) (SweepResult :type "HitResult Structure (by ref)"))
  (set `self.Looping` false)
  (`KismetSystemLibrary.Delay` 0.1)
  (`/Game/MainAssets/CharacterBlueprints/WBP_Arena_UI.ViewTime` (`self.ArenaUIRef`))
  (set `self.CountDown` 3.0)
  (`KismetSystemLibrary.K2_SetTimerDelegate` (delegate `Timer`) 0.1 (`self.Looping`) :!label _label))

(event `self.Box.OnComponentEndOverlap`
  (params (OverlappedComponent :type "PrimitiveComponent Object Reference") (OtherActor :type "Actor Object Reference") (OtherComp :type "PrimitiveComponent Object Reference") (OtherBodyIndex :type Integer))
  (set `self.Looping` true)
  (`KismetSystemLibrary.Delay` 0.1)
  (`/Game/MainAssets/CharacterBlueprints/WBP_Arena_UI.ViewTime` (`self.ArenaUIRef`))
  (goto _label))

(event `Timer`
  (set `self.CountDown` (`KismetMathLibrary.FClamp` (- (`self.CountDown`) 0.1) 0.0 (`self.CountDown`)))
  (if (== (`self.CountDown`) 0.0)
    (`/Engine/EditorBlueprintResources/StandardMacros.DoOnce` false
      (:`Completed`
        (bind _asbp_player_character (cast `/Game/MainAssets/CharacterBlueprints/BP_PlayerCharacter` (`GameplayStatics.GetPlayerCharacter` 0)))
        (`GameplayStatics.ApplyDamage` _asbp_player_character 100.0)))))

(fn `UserConstructionScript`)